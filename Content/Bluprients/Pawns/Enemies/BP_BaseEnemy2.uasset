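; BP_BaseEnemy2 is an enemy Blueprint that constantly moves forward while gradually steering toward the player pawn.
; BeginPlay caches player pawn 0, and Tick moves the actor 5 units along local forward without sweep or delta-time scaling.
; While that pawn is valid, Tick yaws toward it using the look-at difference clamped to ±30 and scaled by delta seconds, limiting turns to 30 degrees per second.
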(event EventBeginPlay
  (|CallParentFunction)
  (Variables|Default|SetPlayerPawn (Game|Player|GetPlayerPawn 0)))

(event EventTick
  (params (DeltaSeconds :type Float%20%28single-precision%29))
  (|CallParentFunction DeltaSeconds)
  (Transformation|AddActorLocalOffset "5.000000, 0, 0" false false)
  (Variables|Default|GetPlayerPawn
    (:then
      (Transformation|AddActorLocalRotation (Math|Rotator|MakeRotator 0.0 0.0 (* (Math|Float|Clamp(Float) (.yaw (Math|Rotator|Delta(Rotator) (Math|Rotator|FindLookatRotation (Transformation|GetActorLocation) (Transformation|GetActorLocation (Variables|Default|GetPlayerPawn))) (Transformation|GetActorRotation))) -3e+01 3e+01) (Utilities|Time|GetWorldDeltaSeconds))) false false))
    (:else)))

(fn ConstructionScript)