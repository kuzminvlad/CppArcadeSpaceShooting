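; BP_PlaygroundBorder is an actor that fits a Trigger box to the visible play area at game start.
; After a half-second delay on BeginPlay, it deprojects the viewport-size screen point to world space for player 0.
; That point's X and Z, plus fixed margins, set the box's X and Y extents, and X also offsets its world location.
; The graph contains no overlap handling.
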(event EventBeginPlay
  (bind _returnvalue (Viewport|GetViewportSize))
  (bind _returnvalue_2 (Game|GetPlayerController 0))
  (bind _worldposition (Class|GameplayStatics|DeprojectScreentoWorld _returnvalue_2 _returnvalue))
  (bind (_x _y _z) (Math|Vector|BreakVector _worldposition))
  (Utilities|FlowControl|Delay 0.5)
  (Components|Box|SetBoxExtent (Variables|Default|GetTrigger) (Math|Vector|MakeVector (+ _x 3e+02) (+ _z 2e+02) 5e+01) true)
  (Transformation|SetWorldLocation (Variables|Default|GetTrigger) (Math|Vector|MakeVector (+ _x 2e+02) 0.0 0.0) false false))

(fn ConstructionScript)